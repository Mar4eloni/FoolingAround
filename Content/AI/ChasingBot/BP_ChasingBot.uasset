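; BP_ChasingBot is an AI-controlled bot that moves toward the first player's pawn when play begins.
; On BeginPlay it runs FindNextPathPoint, then issues a single SimpleMoveToActor through its AI controller.
; FindNextPathPoint computes a synchronous navigation path to the player and draws temporary debug spheres at each point.
; That path is only visualized and does not drive movement.
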(event `self.ReceiveBeginPlay`
  (`self.FindNextPathPoint`)
  (`AIBlueprintHelperLibrary.SimpleMoveToActor` (`AIBlueprintHelperLibrary.GetAIController` self) (`GameplayStatics.GetPlayerPawn` 0)))

(event `FindNextPathPoint`
  (bind _returnvalue (`NavigationSystemV1.FindPathToActorSynchronously` (`self.K2_GetActorLocation`) (`GameplayStatics.GetPlayerPawn` 0) 50.0 null null))
  (for _array_element (`NavigationPath.PathPoints` _returnvalue)
    (`KismetSystemLibrary.DrawDebugSphere` _array_element 20.0 12 (struct :`R` 1.0 :`G` 1.0 :`B` 1.0 :`A` 1.0) 5.0 1.0)))

(fn `UserConstructionScript`)