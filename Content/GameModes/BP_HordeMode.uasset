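; BP_HordeMode is a game mode Blueprint that spawns BP_ChasingBot enemies at locations chosen by an Environment Query when play begins.
; BeginPlay runs EQS_SpawnLocation once in RandomBest25Pct mode and binds to its query-finished event.
; On success, it loops over the returned locations, draws a debug sphere at each, spawns a bot with collision adjustment and prints the bot's name.
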(event `self.ReceiveBeginPlay`
  (bind _returnvalue (`EnvQueryManager.RunEQSQuery` "/Game/AI/EQS_SpawnLocation.EQS_SpawnLocation" self "RandomBest25Pct"))
  (add `EnvQueryInstanceBlueprintWrapper.OnQueryFinishedEvent` _returnvalue (delegate `OnQueryFinishedEvent_Event_0`)))

(event `OnQueryFinishedEvent_Event_0`
  (params (QueryInstance :type "EnvQueryInstanceBlueprintWrapper Object Reference") (QueryStatus :type "EEnvQueryStatus Enum" :default "Processing"))
  (switch `EEnvQueryStatus` QueryStatus
    (:`Success`
      (bind _resultlocations (`EnvQueryInstanceBlueprintWrapper.GetQueryResultsAsLocations` QueryInstance))
      (for _array_element _resultlocations
        (`KismetSystemLibrary.DrawDebugSphere` _array_element 50.0 12 (struct :`R` 1.0 :`G` 0.743591 :`A` 1.0) 2.0 2.0)
        (bind _returnvalue (`|SpawnActorFromClass` "/Game/AI/ChasingBot/BP_ChasingBot.BP_ChasingBot_C" (`KismetMathLibrary.MakeTransform` _array_element) "AdjustIfPossibleButDontSpawnIfColliding" "OverrideRootScale" null null))
        (`KismetSystemLibrary.PrintString` (`KismetSystemLibrary.GetDisplayName` _returnvalue))))))

(fn `UserConstructionScript`)