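; Player character Blueprint that carries a rifle and shows an on-screen crosshair.
; On BeginPlay it spawns BP_Rifle, stores it as CurrentWeapon, snaps it to the mesh's WeaponSocket and adds WBP_CrossHair to the viewport.
; Fire input delegates to CurrentWeapon's Fire.
; Jump input only toggles the IsJumping flag on press and release, with no jump call in this graph.
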(event `self.ReceiveBeginPlay`
  (bind _returnvalue (`|SpawnActorFromClass` "/Game/Weapons/Snipers/BP_Rifle.BP_Rifle_C" (`KismetMathLibrary.MakeTransform` (0.0 0.0 0.0)) "AlwaysSpawn" "OverrideRootScale" self null))
  (set `self.CurrentWeapon` _returnvalue)
  (`self.K2_AttachToComponent` _returnvalue (`self.Mesh`) "WeaponSocket" "SnapToTarget" "SnapToTarget" "SnapToTarget" true)
  (bind _returnvalue_2 (`|CreateWidget` "/Game/UI/WBP_CrossHair.WBP_CrossHair_C"))
  (`UserWidget.AddToViewport` _returnvalue_2 0))

(event `InputAction|Fire`
  (params (Key :type "Key Structure"))
  (:`Pressed`
    (`SWeaponBase.Fire` (`self.CurrentWeapon`))))

(event `InputAction|Jump`
  (params (Key :type "Key Structure"))
  (:`Pressed`
    (set `self.bIsJumping` true))
  (:`Released`
    (set `self.bIsJumping` false)))

(fn `UserConstructionScript`)